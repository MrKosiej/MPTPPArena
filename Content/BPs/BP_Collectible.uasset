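; BP_Collectible is a collectible actor, typed as Weapon or HealthPack, that shows a widget to the local player standing in its overlap area.
; Begin and end overlap with a BP_CombatCharacter toggle the widget's visibility, only when that character is locally controlled.
; The construction script sets the mesh material to match the collectible type.
; The graphs shown contain no pickup logic.
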(event Custom|Local_TriggerVisibility
  (params (ON :type Boolean))
  (Rendering|SetVisibility (Variables|Default|GetWidget) ON true))

(event Collision|EventActorBeginOverlap
  (params (OtherActor :type Actor%20Object%20Reference))
  (bind _asbp_combat_character (Utilities|Casting|CastToBP_CombatCharacter OtherActor))
  (if (Pawn|IsLocallyControlled _asbp_combat_character)
    (CallFunction|LocalTriggerVisibility true)))

(event Collision|EventActorEndOverlap
  (params (OtherActor :type Actor%20Object%20Reference))
  (bind _asbp_combat_character (Utilities|Casting|CastToBP_CombatCharacter OtherActor))
  (if (Pawn|IsLocallyControlled _asbp_combat_character)
    (CallFunction|LocalTriggerVisibility false)))

(fn ConstructionScript
  (Rendering|Material|SetMaterial (Variables|Default|GetStaticMesh) 0 (Utilities|Select :Index (Variables|Default|GetType) :NewEnumerator0 "/Game/Mats/MI_Collectible_Weapon.MI_Collectible_Weapon" :NewEnumerator1 "/Game/Mats/MI_Collectible_HealthPack.MI_Collectible_HealthPack")))